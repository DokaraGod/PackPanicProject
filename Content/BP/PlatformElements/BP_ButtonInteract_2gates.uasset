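; BP_ButtonInteract_2gates is an interactable platform element that removes its set of rope components when used.
; Cube overlap with the third-person character toggles the prompt Widget's visibility, and its dynamic material starts at zero opacity.
; Interact calls the parent logic, plays a scissors sound, and destroys the ropes, Cube and pickup Niagara effect.
; It records the interaction in IsInteracted, which the IntertactButton function returns.
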(event OnComponentBeginOverlap(Cube)
  (params (OverlappedComponent :type Primitive%20Component%20Object%20Reference) (OtherActor :type Actor%20Object%20Reference) (OtherComp :type Primitive%20Component%20Object%20Reference) (OtherBodyIndex :type Integer) (bFromSweep :type Boolean) (SweepResult :type Hit%20Result%20Structure%20%28by%20ref%29))
  (Utilities|Casting|CastToBP_ThirdPersonCharacter OtherActor)
  (Variables|Default|SetIsOverlapping true)
  (CallFunction|NewFunction))

(event OnComponentEndOverlap(Cube)
  (params (OverlappedComponent :type Primitive%20Component%20Object%20Reference) (OtherActor :type Actor%20Object%20Reference) (OtherComp :type Primitive%20Component%20Object%20Reference) (OtherBodyIndex :type Integer))
  (Utilities|Casting|CastToBP_ThirdPersonCharacter OtherActor)
  (Variables|Default|SetIsOverlapping false)
  (CallFunction|NewFunction))

(event EventBeginPlay
  (bind _returnvalue (Rendering|Material|CreateDynamicMaterialInstance (Variables|Default|GetCube) 0 0 "None" :!class /Script/Engine.PrimitiveComponent))
  (Variables|Default|SetMaterial _returnvalue)
  (Rendering|Material|SetScalarParameterValue (Variables|Default|GetMaterial) "Opacity" 0.0 :!class /Script/Engine.MaterialInstanceDynamic))

(event EventInteract
  (Variables|Default|SetIsInteracted true)
  (|CallParentFunction)
  (Audio|PlaySound2D "/Game/Sound/SFX/S_Scissors.S_Scissors" 1.0 1.0 0.0 0 0)
  (CallFunction|DestroyComponents)
  (CallFunction|IntertactButton))

(fn ConstructionScript
  (|CallParentFunction))

(fn IntertactButton
  (return (Variables|Default|GetIsInteracted)))

(fn NewFunction
  (Rendering|SetVisibility (Variables|Default|GetWidget) (Variables|Default|GetIsOverlapping) false))

(fn DestroyComponents
  (Components|DestroyComponent (Variables|Default|GetRopeNew19)))