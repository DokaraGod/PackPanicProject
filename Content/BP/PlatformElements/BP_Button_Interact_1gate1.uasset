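; Interactable button platform element that triggers a linked Claw when used, as a child of a parent interact Blueprint.
; On Interact it runs the parent logic, then fires once via DoOnce, playing a 2D sound and starting a timeline that moves the button cylinder along Z.
; Timeline updates also pass through a one-second delay before calling the Claw's animation.
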(event EventInteract
  (|CallParentFunction)
  (Utilities|FlowControl|DoOnce false
    (:Completed
      (Audio|PlaySound2D "/Game/Sound/SFX/S_Interact.S_Interact" 1.0 1.0 0.0 0 0)
      (bind _newtrack_0 (Timeline|Timeline Play)
        (:Update
          (Transformation|SetRelativeLocation (Variables|Default|GetButton_Cylinder_001) (Math|Vector|MakeVector 0.0 0.0 (* _newtrack_0 1.0)) false false)
          (Utilities|FlowControl|Delay 1.0)
          (Default|ClawAnimation (Variables|Default|GetClaw)))))))

(fn ConstructionScript
  (|CallParentFunction))