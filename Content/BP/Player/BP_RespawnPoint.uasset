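; BP_RespawnPoint is a checkpoint actor that registers itself as the respawn point of any BP_ThirdPersonCharacter overlapping it.
; Every such overlap updates the character's RespawnPoint and prints a "Checkpoint" message.
; A DoOnce limits the activation feedback to the first overlap, showing two point lights, playing a sound and swapping the cylinder to its active material.
; GetSpawnLocRot exposes the Pivot component's world location and rotation as the spawn transform.
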(event Collision|EventActorBeginOverlap
  (params (OtherActor :type Actor%20Object%20Reference))
  (bind _asbp_third_person_character (Utilities|Casting|CastToBP_ThirdPersonCharacter OtherActor))
  (Variables|/Game/BP/Player/BP_ThirdPersonCharacter.BP_ThirdPersonCharacter_C|SetRespawnPoint _asbp_third_person_character self)
  (Development|PrintString "Checkpoint")
  (Utilities|FlowControl|DoOnce false
    (:Completed
      (Rendering|SetVisibility (Variables|Default|GetPointLight1) true false)
      (Audio|PlaySound2D "/Game/Sound/SFX/S_Checkpoint.S_Checkpoint" 1.0 1.0 0.0 0 0)
      (Rendering|Material|SetMaterial (Variables|Default|GetCylinder) 0 "/Game/Assets/MaterialAssets/MaterialCheckpoint/Active/Checkpoint_Active.Checkpoint_Active"))))

(fn ConstructionScript)

(fn GetSpawnLocRot
  (bind _pivot (Variables|Default|GetPivot))
  (return (Transformation|GetWorldLocation _pivot) (Transformation|GetWorldRotation _pivot)))