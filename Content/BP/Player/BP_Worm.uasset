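; BP_Worm is a worm enemy that turns to track the player, attacks when they come close and knocks them back.
; Tick yaws it at a constant rate and, on sphere overlap, plays the attack montage, re-armed after the montage length.
; Mesh overlap with the third-person character launches them away and upward.
; Do-once gates and delays throttle both the attack and the launch.
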(event OnComponentBeginOverlap(Worm_Mesh)
  (params (OverlappedComponent :type Primitive%20Component%20Object%20Reference) (OtherActor :type Actor%20Object%20Reference) (OtherComp :type Primitive%20Component%20Object%20Reference) (OtherBodyIndex :type Integer) (bFromSweep :type Boolean) (SweepResult :type Hit%20Result%20Structure%20%28by%20ref%29))
  (bind _returnvalue (Transformation|GetActorLocation))
  (bind _player (Variables|Default|GetPlayer))
  (bind _returnvalue_2 (Transformation|GetActorLocation _player))
  (bind _returnvalue_3 (- _returnvalue_2 _returnvalue))
  (bind _asbp_third_person_character (Utilities|Casting|CastToBP_ThirdPersonCharacter OtherActor))
  (Utilities|FlowControl|DoOnce false
    (:Completed
      (Character|LaunchCharacter _asbp_third_person_character (* (+ (Math|Vector|Normalize (Math|Vector|MakeVector (.x _returnvalue_3) (.y _returnvalue_3) 0.0)) (Math|Vector|MakeVector 0.0 0.0 (Variables|Default|GetLaunch%20Z))) (Variables|Default|GetLaunch%20Strengh)) false false)
      (Utilities|FlowControl|Delay (Variables|Default|GetLaunch%20Delay))
      (CallFunction|ResetLaunch))))

(event Custom|Re-enableAttack
  (Utilities|FlowControl|DoOnce false) ; enters at Reset
)

(event Custom|ResetLaunch
  (bind _returnvalue (Transformation|GetActorLocation))
  (bind _player (Variables|Default|GetPlayer))
  (bind _returnvalue_2 (Transformation|GetActorLocation _player))
  (bind _returnvalue_3 (- _returnvalue_2 _returnvalue))
  (Utilities|FlowControl|DoOnce false) ; enters at Reset
)

(event EventBeginPlay
  (bind _asbp_third_person_character (Utilities|Casting|CastToBP_ThirdPersonCharacter (Game|Player|GetPlayerPawn 0)))
  (Variables|Default|SetPlayer _asbp_third_person_character))

(event EventTick
  (params (DeltaSeconds :type Float%20%28single-precision%29))
  (CallFunction|LookatPlayer)
  (if (Collision|IsOverlappingActor (Variables|Default|GetSphere) (Variables|Default|GetPlayer) :!class /Script/Engine.PrimitiveComponent)
    (Utilities|FlowControl|DoOnce false
      (:Completed
        (bind _attackanimduration (CallFunction|Attack))
        (Utilities|FlowControl|Delay (+ _attackanimduration 0.2))
        (CallFunction|Re-enableAttack)))))

(fn ConstructionScript)

(fn LookatPlayer
  (Transformation|SetActorRotation (Class|KismetMathLibrary|RInterptoConstant (Transformation|GetActorRotation) (Math|Rotator|MakeRotator 0.0 0.0 (.yaw (Math|Rotator|FindLookatRotation (Transformation|GetActorLocation (Variables|Default|GetPlayer)) (Transformation|GetActorLocation)))) (Utilities|Time|GetWorldDeltaSeconds) (Math|Float|Lerp 1e+02 0.0001 0.0))))

(fn Attack
  (bind _returnvalue (Animation|Montage|MontagePlay (Components|SkeletalMesh|GetAnimInstance (Variables|Default|GetWorm_Mesh)) "/Game/Assets/Worm/Worm_Attack_Montage.Worm_Attack_Montage" 1.0 "MontageLength" 0.0 true))
  (Variables|Default|SetIsAttacking? true)
  (return _returnvalue))

(fn Idle
  (Animation|Montage|MontagePlay (Components|SkeletalMesh|GetAnimInstance (Variables|Default|GetWorm_Mesh)) "/Game/Assets/Worm/Worm_Idle_Montage.Worm_Idle_Montage" 1.0 "MontageLength" 0.0 true))