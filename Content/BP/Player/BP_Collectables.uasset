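; BP_Collectables is a pickup actor that spins idly until a BP_ThirdPersonCharacter overlaps it.
; The first such overlap, gated by DoOnce, starts the collect animation and calls OnCollected with the character, which here only prints a message.
; The CoinCollect timeline drives the Pivot's height, extra spin and scale, then destroys the actor when it finishes.
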(event Custom|OnCollected
  (params (Third%20Person%20Character :type BP%20Third%20Person%20Character%20Object%20Reference))
  (Development|PrintString "Collected collectable"))

(event Custom|PlayCollectAnimation
  (bind (_direction _zmovement _rotationspeed _scale) (Timeline|CoinCollect Play)
    (:Update
      (Transformation|SetRelativeLocation (Variables|Default|GetPivot) (Math|Vector|MakeVector 0.0 0.0 (* _zmovement (Variables|Default|GetAnim_ZDistance))) false false)
      (Transformation|AddRelativeRotation (Variables|Default|GetPivot) (Math|Rotator|MakeRotator 0.0 0.0 (* _rotationspeed (Variables|Default|GetAnim_RotSpeed) (Utilities|Time|GetWorldDeltaSeconds))) false false)
      (Transformation|SetWorldScale3D (Variables|Default|GetPivot) (* _scale "1.000000,1.000000,1.000000")))
    (:Finished
      (Actor|DestroyActor))))

(event Collision|EventActorBeginOverlap
  (params (OtherActor :type Actor%20Object%20Reference))
  (bind _asbp_third_person_character (Utilities|Casting|CastToBP_ThirdPersonCharacter OtherActor))
  (Utilities|FlowControl|DoOnce false
    (:Completed
      (CallFunction|PlayCollectAnimation)
      (CallFunction|OnCollected _asbp_third_person_character))))

(event EventTick
  (params (DeltaSeconds :type Float%20%28single-precision%29))
  (Transformation|AddRelativeRotation (Variables|Default|GetPivot) (Math|Rotator|MakeRotator 0.0 0.0 (* (Variables|Default|GetIdle_RotSpeed) (Utilities|Time|GetWorldDeltaSeconds))) false false))

(fn ConstructionScript)