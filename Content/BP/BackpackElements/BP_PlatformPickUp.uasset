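; Pickup actor, named as a backpack platform element, that shows a prompt widget and can be removed from the world when picked up.
; Collision overlap begin and end show and hide the widget, with no filter on the overlapping actor.
; PickUpObject simply destroys the actor.
; CanGetPickedUp returns true only while the player pawn is not overlapping the separate Box component.
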(event OnComponentBeginOverlap(Collision)
  (params (OverlappedComponent :type Primitive%20Component%20Object%20Reference) (OtherActor :type Actor%20Object%20Reference) (OtherComp :type Primitive%20Component%20Object%20Reference) (OtherBodyIndex :type Integer) (bFromSweep :type Boolean) (SweepResult :type Hit%20Result%20Structure%20%28by%20ref%29))
  (Rendering|SetVisibility (Variables|Default|GetWidget) true false))

(event OnComponentEndOverlap(Collision)
  (params (OverlappedComponent :type Primitive%20Component%20Object%20Reference) (OtherActor :type Actor%20Object%20Reference) (OtherComp :type Primitive%20Component%20Object%20Reference) (OtherBodyIndex :type Integer))
  (Rendering|SetVisibility (Variables|Default|GetWidget) false false))

(event EventPickUpObject
  (Actor|DestroyActor))

(fn ConstructionScript
  (|CallParentFunction))

(fn CanGetPickedUp
  (return (not (Collision|IsOverlappingActor (Variables|Default|GetBox) (Game|Player|GetPlayerPawn 0) :!class /Script/Engine.PrimitiveComponent))))