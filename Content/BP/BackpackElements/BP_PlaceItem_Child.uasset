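; BP_PlaceItem_Child is a backpack-element variant of a place-item Blueprint that animates the opacity of its Painting component when play begins.
; After running the parent BeginPlay, it creates a dynamic material instance on the component's first material slot.
; A timeline then drives that material's Opacity parameter each update while holding Emissive Color at zero.
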(event EventBeginPlay
  (|CallParentFunction)
  (bind _returnvalue (Rendering|Material|CreateDynamicMaterialInstance (Variables|Default|GetPainting) 0 0 "None" :!class /Script/Engine.PrimitiveComponent))
  (Variables|Default|SetMaterialTransparent _returnvalue)
  (bind _newtrack_0 (Timeline|Timeline Play)
    (:Update
      (Rendering|Material|SetScalarParameterValue (Variables|Default|GetMaterialTransparent) "Opacity" _newtrack_0 :!class /Script/Engine.MaterialInstanceDynamic)
      (Rendering|Material|SetScalarParameterValue (Variables|Default|GetMaterialTransparent) "Emissive Color" 0.0 :!class /Script/Engine.MaterialInstanceDynamic))))

(event Collision|EventActorBeginOverlap
  (params (OtherActor :type Actor%20Object%20Reference)))

(event EventTick
  (params (DeltaSeconds :type Float%20%28single-precision%29))
  (|CallParentFunction DeltaSeconds) ; This node is disabled and will not be called.\nDrag off pins to build functionality.
)

(fn ConstructionScript
  (|CallParentFunction))