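; Bounce platform pickup that launches the third-person character on contact and can be picked up, which destroys the actor.
; Hit events with a normal Z of at most 0.1 add BounceStrengh to the character's velocity through LaunchCharacter.
; A DoOnce gate resets after a short delay to prevent repeated launches.
; Collision overlap begin and end show and hide its widget, without checking which actor overlaps.
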(event OnComponentBeginOverlap(Collision)
  (params (OverlappedComponent :type Primitive%20Component%20Object%20Reference) (OtherActor :type Actor%20Object%20Reference) (OtherComp :type Primitive%20Component%20Object%20Reference) (OtherBodyIndex :type Integer) (bFromSweep :type Boolean) (SweepResult :type Hit%20Result%20Structure%20%28by%20ref%29))
  (Rendering|SetVisibility (Variables|Default|GetWidget) true false))

(event OnComponentEndOverlap(Collision)
  (params (OverlappedComponent :type Primitive%20Component%20Object%20Reference) (OtherActor :type Actor%20Object%20Reference) (OtherComp :type Primitive%20Component%20Object%20Reference) (OtherBodyIndex :type Integer))
  (Rendering|SetVisibility (Variables|Default|GetWidget) false false))

(event EventPickUpObject
  (Actor|DestroyActor))

(event Collision|EventHit
  (params (MyComp :type Primitive%20Component%20Object%20Reference) (Other :type Actor%20Object%20Reference) (OtherComp :type Primitive%20Component%20Object%20Reference) (bSelfMoved :type Boolean) (HitLocation :type Vector :default "0, 0, 0") (HitNormal :type Vector :default "0, 0, 0") (NormalImpulse :type Vector :default "0, 0, 0") (Hit :type Hit%20Result%20Structure%20%28by%20ref%29))
  (if (<= (.Z (Math|Vector|BreakVector HitNormal)) 0.1)
    (Utilities|FlowControl|DoOnce false :!label _label
      (:Completed
        (bind _asbp_third_person_character (Utilities|Casting|CastToBP_ThirdPersonCharacter Other))
        (Character|LaunchCharacter _asbp_third_person_character (Variables|Default|GetBounceStrengh) false false)
        (Utilities|FlowControl|Delay 0.2)
        (goto _label Reset)))))

(fn ConstructionScript
  (|CallParentFunction))