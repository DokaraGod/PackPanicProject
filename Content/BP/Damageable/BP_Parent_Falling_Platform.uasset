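; Parent falling platform that shakes and drops when the third-person character overlaps it.
; A FallingAnimation timeline drifts the Pivot along Y and yaws it, with tracks named opposite to what they drive, then Cube simulates physics after a short delay.
; After RespawnDelay, physics stops and only Pivot's relative transform is zeroed.
; Both DoOnce gates never reset, so it triggers once, and the saved PlatformPos is unused.
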(event Custom|PlatformHit
  (Utilities|FlowControl|DoOnce false
    (:Completed
      (bind (_direction _rotation _location) (Timeline|FallingAnimation Play)
        (:Update
          (Transformation|AddRelativeLocation (Variables|Default|GetPivot) (Math|Vector|MakeVector 0.0 (* _rotation (Utilities|Time|GetWorldDeltaSeconds) (Variables|Default|GetRotation)) 0.0) false false)
          (Transformation|SetRelativeRotation (Variables|Default|GetPivot) (Math|Rotator|MakeRotator 0.0 0.0 (* _location (Variables|Default|GetBreaking))) false false))
        (:Finished
          (Utilities|FlowControl|Delay 0.5)
          (Physics|SetSimulatePhysics (Variables|Default|GetCube) true)
          (Utilities|FlowControl|Delay (Variables|Default|GetRespawnDelay))
          (Physics|SetSimulatePhysics (Variables|Default|GetCube) false)
          (Transformation|SetRelativeRotation (Variables|Default|GetPivot) "0, 0, 0" false false)
          (Transformation|SetRelativeLocation (Variables|Default|GetPivot) "0, 0, 0" false false))))))

(event Collision|EventActorBeginOverlap
  (params (OtherActor :type Actor%20Object%20Reference))
  (Utilities|Casting|CastToBP_ThirdPersonCharacter OtherActor)
  (Utilities|FlowControl|DoOnce false
    (:Completed
      (Variables|Default|SetPlatformPos (Transformation|GetWorldTransform (Variables|Default|GetPivot)))
      (CallFunction|PlatformHit))))

(fn ConstructionScript)