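; Damageable actor component that tracks health for its owning actor and destroys that actor when health reaches zero.
; BeginPlay stores starting Health as MaxHealth, which feeds a clamped health fraction getter.
; TakeDamage subtracts health, broadcasts OnTookDamage, then checks for death.
; A hit handler routes to TakeDamage with a set CollisionDamage, but its binding to the owner's OnActorHit is never executed.
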(event Custom|TakeCollisonDamage
  (CallFunction|TakeDamage (Variables|Default|GetCollisionDamage)))

(event Custom|TakeDamage
  (params (DamageAmount :type Float%20%28double-precision%29))
  (bind _output_get (Variables|Default|SetHealth (- (Variables|Default|GetHealth) DamageAmount)))
  (Default|CallOnTookDamage)
  (if (<= _output_get 0.0)
    (CallFunction|Die)))

(event Custom|OnActorHit_Event
  (params (SelfActor :type Actor%20Object%20Reference) (OtherActor :type Actor%20Object%20Reference) (NormalImpulse :type Vector) (Hit :type Hit%20Result%20Structure%20%28by%20ref%29))
  (CallFunction|TakeCollisonDamage))

(event EventBeginPlay
  (Variables|Default|SetMaxHealth (Variables|Default|GetHealth)))

(fn GetHealthPercentage
  (return (Math|Float|Clamp(Float) (/ (Variables|Default|GetHealth) (Variables|Default|GetMaxHealth)))))

(fn Die
  (Actor|DestroyActor (Components|GetOwner)))