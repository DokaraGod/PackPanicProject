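; Falling platform Blueprint that replaces itself with a fresh copy after the player character overlaps it.
; Overlap first runs the parent's handler, then a DoOnce gate lets only the first BP_ThirdPersonCharacter contact start the respawn timer.
; After RespawnDelay plus a one-second margin, it spawns an instance of its own class at the PlatformPos transform and destroys itself.
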(event Collision|EventActorBeginOverlap
  (params (OtherActor :type Actor%20Object%20Reference))
  (|CallParentFunction OtherActor)
  (Utilities|Casting|CastToBP_ThirdPersonCharacter OtherActor)
  (Utilities|FlowControl|DoOnce false
    (:Completed
      (Utilities|FlowControl|Delay (+ (Variables|Default|GetRespawnDelay) 1.0))
      (Game|SpawnActorfromClass (Utilities|GetClass self) (Variables|Default|GetPlatformPos) "Undefined" "MultiplyWithRoot" 0 0)
      (Actor|DestroyActor))))

(fn ConstructionScript
  (|CallParentFunction))